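; BP_Player is the player-controlled ship or character that moves on a plane and fires lasers.
; On BeginPlay it switches to flying movement and stores the capsule's starting transform, which is not read in this graph.
; The Up and Right axes drive movement along world X and negative Z.
; Pressing Shoot spawns a BP_Player_Laser at the LaserCannon component's transform.
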(event `self.ReceiveBeginPlay`
  (`CharacterMovementComponent.SetMovementMode` (`self.CharacterMovement`) "MOVE_Flying" 0)
  (set `self.StartPosition` (`SceneComponent.K2_GetComponentToWorld` (`self.CapsuleComponent`))))

(event `InputAxis|Up`
  (params (AxisValue :type "Float (single-precision)"))
  (`self.AddMovementInput` (1.0 0.0 0.0) AxisValue))

(event `InputAxis|Right`
  (params (AxisValue :type "Float (single-precision)"))
  (`self.AddMovementInput` (0.0 0.0 -1.0) AxisValue))

(event `InputAction|Shoot`
  (params (Key :type "Key Structure"))
  (:`Pressed`
    (`|SpawnActorFromClass` "/Game/Blueprints/BP_Player_Laser.BP_Player_Laser_C" (`SceneComponent.K2_GetComponentToWorld` (`self.LaserCannon`)) "Undefined" "MultiplyWithRoot" null null)))

(fn `UserConstructionScript`)