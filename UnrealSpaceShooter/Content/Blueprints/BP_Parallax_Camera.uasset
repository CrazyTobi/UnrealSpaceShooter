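; BP_Parallax_Camera is a camera actor that scrolls a background plane's material to create a parallax effect.
; On BeginPlay, if BP_Player exists, it creates a dynamic instance of M_Parallax_Material on the plane and becomes the player's view target.
; Each Tick accumulates an offset from delta time and BackgroundSpeed and writes it to the material's Offset parameter.
; The scroll rate is independent of player movement.
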(event `self.ReceiveBeginPlay`
  ;[1 1 1] Setting Variables for parallax camera
  (bind _returnvalue (`GameplayStatics.GetActorOfClass` "/Game/Blueprints/BP_Player.BP_Player_C"))
  (set `self.Player` _returnvalue)
  (`/Engine/EditorBlueprintResources/StandardMacros.IsValid` (`self.Player`)
    (:`Is Valid`
      (bind _returnvalue_2 (`PrimitiveComponent.CreateDynamicMaterialInstance` (`self.Plane`) 0 "/Game/Assets/Materials/M_Parallax_Material.M_Parallax_Material" "None"))
      (set `self.MID` _returnvalue_2)
      (`PlayerController.SetViewTargetWithBlend` (`GameplayStatics.GetPlayerController` 0) self 0.0 "VTBlend_Linear" 0.0 false))))

(event `self.ReceiveTick`
  (params (DeltaSeconds :type "Float (single-precision)"))
  ;[1 1 1] Implment Parallax Camera
  (set `self.Delta` (* (`GameplayStatics.GetWorldDeltaSeconds`) (`KismetMathLibrary.VSize` (* (`KismetMathLibrary.Vector_Normal2D` (`KismetMathLibrary.MakeVector` 5.0)) (`self.BackgroundSpeed`)))))
  (set `self.Delta` (+ (`self.Delta`) 0.0))
  (set `self.CurrentOffset` (+ (`self.CurrentOffset`) (`self.Delta`)))
  (`MaterialInstanceDynamic.SetScalarParameterValue` (`self.MID`) "Offset" (`self.CurrentOffset`)))

(fn `UserConstructionScript`)