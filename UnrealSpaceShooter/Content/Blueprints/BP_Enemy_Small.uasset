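; BP_Enemy_Small is a small enemy with a Paper2D flipbook sprite that turns to match its movement direction.
; Every Tick reads the capsule's X velocity and calls FlipSpriteDown when it is negative, otherwise FlipSpriteUp.
; Both functions flip the sprite by setting the flipbook's relative rotation to opposite 90-degree angles.
; Zero X velocity counts as positive, so a stopped enemy always reverts to the Up orientation.
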(event `self.ReceiveTick`
  (params (DeltaSeconds :type "Float (single-precision)"))
  (bind _returnvalue_x (`KismetMathLibrary.BreakVector` (`SceneComponent.GetComponentVelocity` (`self.Capsule`))))
  ;[1 1 1] Flip enemy sprites
  (if (< _returnvalue_x 0.0)
    (`self.FlipSpriteDown`)
    (else
      (`self.FlipSpriteUp`))))

(fn `FlipSpriteDown`
  (`SceneComponent.K2_SetRelativeRotation` (`self.PaperFlipbook`) (struct :`Pitch` -90.0) false false))

(fn `FlipSpriteUp`
  (`SceneComponent.K2_SetRelativeRotation` (`self.PaperFlipbook`) (struct :`Pitch` 90.0) false false))

(fn `UserConstructionScript`)